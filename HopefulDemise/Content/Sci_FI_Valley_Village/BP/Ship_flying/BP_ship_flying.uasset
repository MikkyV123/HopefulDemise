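; Ambient flying ship actor that moves a ship mesh along an editable spline path.
; Tick advances a distance by speed, delta time and a fixed per-frame step, then snaps the mesh to that spline location and rotation.
; When looping is on, a check after a Delay restarts the distance near the spline's start once it passes the end.
; The construction script's per-segment loop is empty, with its spline sampling nodes left unused.
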(event EventBeginPlay)

(event EventTick
  (params (DeltaSeconds :type Float%20%28single-precision%29))
  (Variables|Default|SetDistance (+ (* DeltaSeconds (Variables|Default|GetSpeed)) (Variables|Default|GetDistance) 1.0))
  (Transformation|SetRelativeTransform (Variables|Default|GetSM_ship) (Math|Transform|MakeTransform (.location (Spline|GetTransformatDistanceAlongSpline (Variables|Default|GetSpline) (Variables|Default|GetDistance) "Local" false)) (.rotation (Spline|GetTransformatDistanceAlongSpline (Variables|Default|GetSpline) (Variables|Default|GetDistance) "Local" false)) (Variables|/Script/Engine.SceneComponent|GetRelativeScale3D (Variables|Default|GetSM_ship))) false false)
  (Utilities|FlowControl|Delay (Variables|Default|GetDuration))
  (if (Variables|Default|GetIslooping)
    (if (> (Variables|Default|GetDistance) (Spline|GetSplineLength (Variables|Default|GetSpline)))
      (Variables|Default|SetDistance 1.0))))

(fn ConstructionScript
  (for _index (range 0 (- (Math|Float|Truncate (/ (Spline|GetSplineLength (Variables|Default|GetSpline)) (Variables|Default|GetLength))) 1))
    _))