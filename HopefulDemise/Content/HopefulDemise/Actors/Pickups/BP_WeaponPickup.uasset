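; BP_WeaponPickup is a weapon pickup actor that the player collects by interacting with it.
; On Interact, it tells the interacting player to spawn the weapon set in its WeaponToSpawn variable, then destroys itself.
; It has no active BeginPlay, overlap or Tick logic, and its construction script only calls the parent.
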(event EventBeginPlay
  (|CallParentFunction) ; This node is disabled and will not be called.\nDrag off pins to build functionality.
)

(event Collision|EventActorBeginOverlap
  (params (OtherActor :type Actor%20Object%20Reference))
  (|CallParentFunction OtherActor) ; This node is disabled and will not be called.\nDrag off pins to build functionality.
)

(event EventTick
  (params (DeltaSeconds :type Float%20%28single-precision%29))
  (|CallParentFunction DeltaSeconds) ; This node is disabled and will not be called.\nDrag off pins to build functionality.
)

(event EventInteract
  (params (Player :type BP%20Ettore%20Object%20Reference))
  (Default|SpawnWeapon Player (Variables|Default|GetWeapon%20To%20Spawn))
  (Actor|DestroyActor))

(fn ConstructionScript
  (|CallParentFunction))