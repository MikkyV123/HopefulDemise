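; BP_AKM is the AKM weapon actor, providing the gun's firing audio.
; Its Fire event plays the AKShot sound at reduced volume at the WeaponModel's location, using no named socket.
; The graph has no other active logic: BeginPlay, overlap and Tick are disabled stubs, and the construction script only calls its parent.
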(event EventBeginPlay
  (|CallParentFunction) ; This node is disabled and will not be called.\nDrag off pins to build functionality.
)

(event Collision|EventActorBeginOverlap
  (params (OtherActor :type Actor%20Object%20Reference))
  (|CallParentFunction OtherActor) ; This node is disabled and will not be called.\nDrag off pins to build functionality.
)

(event EventTick
  (params (DeltaSeconds :type Float%20%28single-precision%29))
  (|CallParentFunction DeltaSeconds) ; This node is disabled and will not be called.\nDrag off pins to build functionality.
)

(event EventFire
  (Audio|PlaySoundatLocation "/Game/HopefulDemise/Audio/AKShot.AKShot" (Transformation|GetSocketLocation (Variables|Default|GetWeaponModel) "None") "0, 0, 0" 0.5 1.0 0.0 0 0 0 0))

(fn ConstructionScript
  (|CallParentFunction))