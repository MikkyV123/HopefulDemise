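; BP_ZiplineMovementActor is a temporary helper actor that carries a player along a zipline from start to end.
; A RealConstructor event stands in for a constructor, storing the player, speed and endpoints, with a standard offset added to both points.
; It plays a timeline at a rate set by MoveSpeed, lerping the player's location without sweep each update, then destroys itself on finish.
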(event Custom|RealConstructor
  (params (MoveSpeed :type Float%20%28double-precision%29) (ZiplineStartPos :type Vector) (ZiplineEndPos :type Vector) (Player :type BP%20First%20Person%20Character%20Object%20Reference))
  (bind _standardziplineoffset (Variables|Default|GetStandardZiplineOffset))
  ;[1 1 1] I think there was a way to make a "proper" constructor to do what I intended but I think I missed it
  (Variables|Default|SetMoveSpeed MoveSpeed)
  (Variables|Default|SetZiplineStartPos (+ ZiplineStartPos _standardziplineoffset))
  (Variables|Default|SetZiplineEndPos (+ ZiplineEndPos _standardziplineoffset))
  (Variables|Default|SetPlayer Player)
  ;[1 1 1] Create the movement timeline for interpolating player position on the zipline
  (Components|Timeline|SetPlayRate (Variables|Default|GetZiplineMovementTimeline) (Variables|Default|GetMoveSpeed))
  (bind _ziplineposition (Timeline|ZiplineMovementTimeline PlayFromStart)
    (:Update
      ;[1 1 1] Move the player
      (Transformation|SetActorLocation (Variables|Default|GetPlayer) (Math|Vector|Lerp(Vector) (Variables|Default|GetZiplineStartPos) (Variables|Default|GetZiplineEndPos) _ziplineposition) false false))
    (:Finished
      (Actor|DestroyActor) ; Destroy when done
    )))

(fn ConstructionScript)