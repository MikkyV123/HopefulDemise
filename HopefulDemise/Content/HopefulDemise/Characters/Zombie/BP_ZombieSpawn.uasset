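; BP_ZombieSpawn is a round-based zombie enemy that chases and punches the player, BP_Ettore.
; Pawn sensing sets the target, a timeline turns the zombie toward it, and an AI MoveTo loop triggers montage attacks with delayed damage.
; Point and radial damage reduce HP.
; Death ragdolls it with a directional impulse, updates the player's zombie count and round-end check, and sometimes drops max ammo before delayed despawn.
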(event OnSeePawn(PawnSensing)
  (params (Pawn :type Pawn%20Object%20Reference))
  ;[1 1 1] Pawn Sensing, Can The Zombie See The Player
  (bind _asbp_ettore (Utilities|Casting|CastToBP_Ettore Pawn))
  (Variables|Default|SetAs%20BP%20Ettore _asbp_ettore)
  (CallFunction|RunAfterPlayer)
  (Variables|Default|Setis%20seeing%20player true))

(event Custom|MarkZombieForDestruction
  ;[1 1 1] Marking Zombie For Destruction (Destroy Actor with Despawn Time)
  (if (<= (Math|Random|RandomInteger 100) 4)
    (Game|SpawnActorfromClass "/Game/HopefulDemise/Actors/BP_MaxAmmo.BP_MaxAmmo_C" (Math|Transform|MakeTransform (Math|Transform|TransformLocation (Math|Transform|MakeTransform "0.000000,0.000000,80.000000" "0, 0, 0" "1.000000,1.000000,1.000000") (Transformation|GetWorldLocation (Variables|Character|GetMesh))) "0, 0, 0" "1.000000,1.000000,1.000000") "Undefined" "MultiplyWithRoot" 0 0)
    (Utilities|FlowControl|Delay (Variables|Default|GetDespawnTime))
    (Actor|DestroyActor)
    (else
      (Utilities|FlowControl|Delay (Variables|Default|GetDespawnTime))
      (Actor|DestroyActor))))

(event Custom|Run%20After%20Player
  (Utilities|FlowControl|DoOnce false
    (:Completed
      (Utilities|FlowControl|Sequence
        (:then_0
          (bind _newtrack_0 (Timeline|Timeline PlayFromStart)
            (:Update
              (bind _output_get (Variables|Default|SetNew%20Track%200 _newtrack_0))
              (bind _is_rotated (CallFunction|RotatingTowardsPlayer _output_get))
              (Variables|Default|SetIs%20Rotated _is_rotated))))
        (:then_1
          (Variables|/Script/Engine.CharacterMovementComponent|SetMaxWalkSpeed (Variables|Character|GetCharacterMovement) 4e+02)
          (AI|AIMoveTo self "0, 0, 0" (Variables|Default|GetAs%20BP%20Ettore) 1.0 false
            (:OnSuccess
              (if (Variables|Default|GetAlive)
                (Variables|Default|SetCan%20Damage true)
                ;[1 1 1] How Fast Can Zombie Attack
                (bind _hitting_player (CallFunction|ZombieAttack))
                (Variables|Default|SetAttacking%20Player _hitting_player)
                (Utilities|FlowControl|Delay 0.85)
                (if (Variables|Default|GetAlive)
                  (bind _asbp_ettore (Utilities|Casting|CastToBP_Ettore (Game|Player|GetPlayerPawn 0)))
                  (Game|Damage|ApplyDamage _asbp_ettore 2e+01 0 self)
                  (Variables|Default|SetAttacking%20Player false)
                  (CallFunction|MovetoPlayer))))
            (:OnFail
              (Variables|Default|SetAttacking%20Player false)
              (CallFunction|MovetoPlayer))))))))

(event Custom|Move%20To%20Player
  (AI|AIMoveTo self "0, 0, 0" (Variables|Default|GetAs%20BP%20Ettore) 1.0 false
    (:OnSuccess
      (if (Variables|Default|GetAlive)
        (Variables|Default|SetCan%20Damage true)
        ;[1 1 1] How Fast Can Zombie Attack
        (bind _hitting_player (CallFunction|ZombieAttack))
        (Variables|Default|SetAttacking%20Player _hitting_player)
        (Utilities|FlowControl|Delay 0.85)
        (if (Variables|Default|GetAlive)
          (bind _asbp_ettore (Utilities|Casting|CastToBP_Ettore (Game|Player|GetPlayerPawn 0)))
          (Game|Damage|ApplyDamage _asbp_ettore 2e+01 0 self)
          (Variables|Default|SetAttacking%20Player false)
          (CallFunction|MovetoPlayer))))
    (:OnFail
      (Variables|Default|SetAttacking%20Player false)
      (CallFunction|MovetoPlayer))))

(event EventBeginPlay
  (Utilities|FlowControl|Sequence
    (:then_0
      (Transformation|AttachComponentToComponent (Variables|Default|GetHitting%20Collision) 0 "CollisionSocket" "SnapToTarget" "SnapToTarget" "SnapToTarget" true)
      (Variables|Default|SetAlive true))
    (:then_1
      (Animation|PlayAnimMontage "/Game/HopefulDemise/Animations/Zombie/Zombie_AnimM.Zombie_AnimM" 1.0 "None")
      (CallFunction|RunAfterPlayer))))

(event Game|Damage|EventPointDamage
  (params (Damage :type Float%20%28single-precision%29) (DamageType :type Damage%20Type%20Object%20Reference) (HitLocation :type Vector :default "0, 0, 0") (HitNormal :type Vector :default "0, 0, 0") (HitComponent :type Primitive%20Component%20Object%20Reference) (BoneName :type Name :default "None") (ShotFromDirection :type Vector :default "0, 0, 0") (InstigatedBy :type Controller%20Object%20Reference) (DamageCauser :type Actor%20Object%20Reference) (HitInfo :type Hit%20Result%20Structure%20%28by%20ref%29))
  (if (Variables|Default|GetIs%20Rotated)
    (bind _dead (CallFunction|SubtractHP Damage :!label _label))
    (if _dead
      (Utilities|FlowControl|DoOnce (not _dead)
        (:Completed
          (Variables|Default|SetAlive false)
          (CallFunction|RagdollZombie)
          (CallFunction|ApplyPushForcetoZombie ShotFromDirection Damage)
          (CallFunction|MarkZombieforDestruction))))
    (else
      ;[1 1 1] If Shot Zombie will turn around
      (Utilities|FlowControl|Sequence
        (:then_0
          (bind _newtrack_0 (Timeline|Timeline PlayFromStart)
            (:Update
              (bind _output_get (Variables|Default|SetNew%20Track%200 _newtrack_0))
              (bind _is_rotated (CallFunction|RotatingTowardsPlayer _output_get))
              (Variables|Default|SetIs%20Rotated _is_rotated))))
        (:then_1
          (CallFunction|MovetoPlayer)
          (goto _label))))))

(event Game|Damage|EventRadialDamage
  (params (DamageReceived :type Float%20%28single-precision%29) (DamageType :type Damage%20Type%20Object%20Reference) (Origin :type Vector :default "0, 0, 0") (HitInfo :type Hit%20Result%20Structure%20%28by%20ref%29) (InstigatedBy :type Controller%20Object%20Reference) (DamageCauser :type Actor%20Object%20Reference))
  (bind _dead (CallFunction|SubtractHP DamageReceived))
  (if _dead
    (Variables|Default|SetAlive false)
    (CallFunction|RagdollZombie)
    (CallFunction|ApplyPushForcetoZombie (Math|Vector|Normalize (- (Transformation|GetWorldLocation (Variables|Character|GetMesh)) Origin)) DamageReceived)
    (CallFunction|MarkZombieforDestruction)))

(fn ConstructionScript)

(fn RagdollZombie
  (bind _capsulecomponent (Variables|Collision|GetCapsuleComponent))
  (Physics|SetSimulatePhysics (Variables|Character|GetMesh) true)
  (Variables|Default|SetAlive false)
  (Collision|SetCollisionResponsetoAllChannels _capsulecomponent "ECR_Ignore")
  (Transformation|SetMobility _capsulecomponent "Movable")
  (bind _asbp_ettore (Utilities|Casting|CastToBP_Ettore (Game|GetPlayerCharacter 0)))
  (Math|Integer|DecrementInt (Variables|/Game/HopefulDemise/Characters/Ettore/BP_Ettore.BP_Ettore_C|GetZombies%20Alive _asbp_ettore)
    (:%20%20
      (Default|CheckifRoundEnd _asbp_ettore)
      (Development|PrintString (Utilities|String|ToString(Integer) (Variables|/Game/HopefulDemise/Characters/Ettore/BP_Ettore.BP_Ettore_C|GetZombies%20Alive _asbp_ettore)))
      (return))))

(fn ApplyPushForcetoZombie
  (params (From :type Vector) (Damage :type Float%20%28double-precision%29))
  (Physics|AddImpulse (Variables|Character|GetMesh) (* From Damage (Variables|Default|GetExplosionForceMultiplier)) "None" false)
  (return))

(fn SubtractHP
  (params (Damage :type Float%20%28double-precision%29))
  (bind _output_get (Variables|Default|SetHP (- (Variables|Default|GetHP) Damage)))
  (return (<= _output_get 0.0)))

(fn ZombieAttack
  (bind _hitting_collision (Variables|Default|GetHitting%20Collision))
  (bind _returnvalue (Collision|IsOverlappingActor _hitting_collision 0 :!class /Script/Engine.PrimitiveComponent))
  (Animation|PlayAnimMontage "/Game/HopefulDemise/Animations/Zombie/ZombiePunch_AM.ZombiePunch_AM" 2.0 "None")
  (if (Variables|Default|GetAlive)
    (if _returnvalue
      (return _returnvalue))))

(fn RotatingTowardsPlayer
  (params (Alpha :type Float%20%28single-precision%29))
  (bind _asbp_ettore (Utilities|Casting|CastToBP_Ettore (Game|GetPlayerCharacter 0)))
  (bind _returnvalue (Transformation|SetActorRotation (Math|Rotator|Lerp(Rotator) (Transformation|GetActorRotation) (Math|Rotator|FindLookatRotation (Transformation|GetActorLocation) (Transformation|GetActorLocation _asbp_ettore)) Alpha true)))
  (return _returnvalue))