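; Zombie enemy character that roams the navmesh and permanently switches to chasing the player once spotted.
; Roaming loops AIMoveTo to random reachable points, playing a montage on each arrival.
; PawnSensing triggers a one-time chase: a Timeline turns it toward the player, walk speed rises, and AIMoveTo repeats, playing a punch montage on arrival.
; The speed and DoOnce reset is unconnected, and no damage is applied here.
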(event OnSeePawn(PawnSensing)
  (params (Pawn :type Pawn%20Object%20Reference))
  ;[1 1 1] Pawn Sensing, Can The Zombie See The Player
  (bind _asbp_first_person_character (Utilities|Casting|CastToBP_FirstPersonCharacter Pawn))
  (Variables|Default|SetAs%20BP%20First%20Person%20Character _asbp_first_person_character)
  (CallFunction|RunAfterPlayer)
  (Variables|Default|Setis%20seeing%20player true))

(event Custom|Start%20Roaming
  ;[1 1 1] Zombie Roaming Code
  (bind _randomlocation (Class|NavigationSystemV1|GetRandomLocationinNavigableRadius (Transformation|GetActorLocation) 5e+03 0 0))
  (AI|AIMoveTo self _randomlocation 0 7e+01 false
    (:OnSuccess
      (bind _returnvalue (Animation|PlayAnimMontage "/Game/HopefulDemise/Animations/Zombie/Zombie_AnimM.Zombie_AnimM" 1.0 "None"))
      (Utilities|FlowControl|Delay _returnvalue))
    (:OnFail
      _))
  (if (not (Variables|Default|Getis%20seeing%20player))
    (CallFunction|StartRoaming)))

(event Custom|Run%20After%20Player
  (Utilities|FlowControl|DoOnce false
    (:Completed
      (Utilities|FlowControl|Sequence
        (:then_0
          (bind _newtrack_0 (Timeline|Timeline PlayFromStart)
            (:Update
              (Transformation|SetActorRotation (Math|Rotator|Lerp(Rotator) (Transformation|GetActorRotation) (Math|Rotator|FindLookatRotation (Transformation|GetActorLocation) (Transformation|GetActorLocation (Variables|Default|GetAs%20BP%20First%20Person%20Character))) _newtrack_0)))))
        (:then_1
          (Variables|/Script/Engine.CharacterMovementComponent|SetMaxWalkSpeed (Variables|Character|GetCharacterMovement) 4e+02)
          (AI|AIMoveTo self "0, 0, 0" (Variables|Default|GetAs%20BP%20First%20Person%20Character) 5.0 false
            (:OnSuccess
              ;[1 1 1] How Fast Can Zombie Attack
              (Animation|PlayAnimMontage "/Game/HopefulDemise/Animations/Zombie/ZombiePunch_AM.ZombiePunch_AM" 2.0 "None")
              (Utilities|FlowControl|Delay 1.45)
              (CallFunction|MovetoPlayer))
            (:OnFail
              (CallFunction|MovetoPlayer))))))))

(event Custom|Move%20To%20Player
  (AI|AIMoveTo self "0, 0, 0" (Variables|Default|GetAs%20BP%20First%20Person%20Character) 5.0 false
    (:OnSuccess
      ;[1 1 1] How Fast Can Zombie Attack
      (Animation|PlayAnimMontage "/Game/HopefulDemise/Animations/Zombie/ZombiePunch_AM.ZombiePunch_AM" 2.0 "None")
      (Utilities|FlowControl|Delay 1.45)
      (CallFunction|MovetoPlayer))
    (:OnFail
      (CallFunction|MovetoPlayer))))

(event EventBeginPlay
  ;[1 1 1] Zombie Roaming Code
  (bind _randomlocation (Class|NavigationSystemV1|GetRandomLocationinNavigableRadius (Transformation|GetActorLocation) 5e+03 0 0))
  (AI|AIMoveTo self _randomlocation 0 7e+01 false
    (:OnSuccess
      (bind _returnvalue (Animation|PlayAnimMontage "/Game/HopefulDemise/Animations/Zombie/Zombie_AnimM.Zombie_AnimM" 1.0 "None"))
      (Utilities|FlowControl|Delay _returnvalue))
    (:OnFail
      _))
  (if (not (Variables|Default|Getis%20seeing%20player))
    (CallFunction|StartRoaming)))

(fn ConstructionScript)